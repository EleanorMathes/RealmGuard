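; BP_CoreHealthPickup is a pickup that restores health to the base when the player touches it.
; When the player character overlaps its Sphere1 component, it plays a pickup sound at its location and destroys itself.
; It then finds the first BP_Base via GetAllActorsOfClass and adds a fixed amount to BaseHealth, capped at BaseMaxHealth.
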(event `self.Sphere1.OnComponentBeginOverlap`
  (params (OverlappedComponent :type "PrimitiveComponent Object Reference") (OtherActor :type "Actor Object Reference") (OtherComp :type "PrimitiveComponent Object Reference") (OtherBodyIndex :type Integer) (bFromSweep :type Boolean) (SweepResult :type "HitResult Structure (by ref)"))
  (if (== OtherActor (`GameplayStatics.GetPlayerCharacter` 0))
    (`GameplayStatics.PlaySoundAtLocation` "/Game/RealmGuard/SFX/Enemy/Pickup.Pickup" (`self.K2_GetActorLocation`) (struct) 1.0 1.0 0.0 null null null null)
    (`self.K2_DestroyActor`)
    (bind _outactors (`GameplayStatics.GetAllActorsOfClass` "/Game/RealmGuard/Base/BP_Base.BP_Base_C"))
    (bind _output (`|GetArrayItem` _outactors))
    (set `/Game/RealmGuard/Base/BP_Base.BaseHealth` (+ (`/Game/RealmGuard/Base/BP_Base.BaseHealth` _output) 15.0) _output)
    (bind _basemaxhealth (`/Game/RealmGuard/Base/BP_Base.BaseMaxHealth` _output))
    (if (>= (`/Game/RealmGuard/Base/BP_Base.BaseHealth` _output) _basemaxhealth)
      (set `/Game/RealmGuard/Base/BP_Base.BaseHealth` _basemaxhealth _output))))

(fn `UserConstructionScript`)