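; BP_HealthPickup is a pickup actor that restores health to the player in RealmGuard.
; When the player character overlaps its Sphere1 component, it casts to BP_ThirdPersonCharacter and adds a fixed amount to Health, capped at a hardcoded maximum.
; The graph neither destroys nor disables the pickup afterward, so each new overlap heals again.
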(event `self.Sphere1.OnComponentBeginOverlap`
  (params (OverlappedComponent :type "PrimitiveComponent Object Reference") (OtherActor :type "Actor Object Reference") (OtherComp :type "PrimitiveComponent Object Reference") (OtherBodyIndex :type Integer) (bFromSweep :type Boolean) (SweepResult :type "HitResult Structure (by ref)"))
  (bind _returnvalue (`GameplayStatics.GetPlayerCharacter` 0))
  (if (== OtherActor _returnvalue)
    (bind _asbp_third_person_character (cast `/Game/ThirdPerson/Blueprints/BP_ThirdPersonCharacter` _returnvalue))
    (set `/Game/ThirdPerson/Blueprints/BP_ThirdPersonCharacter.health` (+ (`/Game/ThirdPerson/Blueprints/BP_ThirdPersonCharacter.health` _asbp_third_person_character) 25.0) _asbp_third_person_character)
    (if (> (`/Game/ThirdPerson/Blueprints/BP_ThirdPersonCharacter.health` _asbp_third_person_character) 100.0)
      (set `/Game/ThirdPerson/Blueprints/BP_ThirdPersonCharacter.health` 100.0 _asbp_third_person_character))))

(fn `UserConstructionScript`)