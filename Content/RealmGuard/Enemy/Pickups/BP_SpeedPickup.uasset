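; BP_SpeedPickup is a pickup that grants the player a temporary speed boost on overlapping its sphere.
; It plays a pickup sound, destroys itself, then raises WalkSpeed and SprintSpreed on BP_ThirdPersonCharacter.
; A Delay is meant to restore fixed default speeds afterward, but it follows DestroyActor on the same actor, so that reset is unlikely to run.
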(event `self.Sphere1.OnComponentBeginOverlap`
  (params (OverlappedComponent :type "PrimitiveComponent Object Reference") (OtherActor :type "Actor Object Reference") (OtherComp :type "PrimitiveComponent Object Reference") (OtherBodyIndex :type Integer) (bFromSweep :type Boolean) (SweepResult :type "HitResult Structure (by ref)"))
  (bind _returnvalue (`GameplayStatics.GetPlayerCharacter` 0))
  (if (== OtherActor _returnvalue)
    (`GameplayStatics.PlaySoundAtLocation` "/Game/RealmGuard/SFX/Enemy/Pickup.Pickup" (`self.K2_GetActorLocation`) (struct) 1.0 1.0 0.0 null null null null)
    (`self.K2_DestroyActor`)
    (bind _asbp_third_person_character (cast `/Game/ThirdPerson/Blueprints/BP_ThirdPersonCharacter` _returnvalue))
    (set `/Game/ThirdPerson/Blueprints/BP_ThirdPersonCharacter.WalkSpeed` 900.0 _asbp_third_person_character)
    (set `/Game/ThirdPerson/Blueprints/BP_ThirdPersonCharacter.SprintSpreed` 1350.0 _asbp_third_person_character)
    (`KismetSystemLibrary.Delay` 20.0)
    (set `/Game/ThirdPerson/Blueprints/BP_ThirdPersonCharacter.WalkSpeed` 450.0 _asbp_third_person_character)
    (set `/Game/ThirdPerson/Blueprints/BP_ThirdPersonCharacter.SprintSpreed` 675.0 _asbp_third_person_character)))

(fn `UserConstructionScript`)