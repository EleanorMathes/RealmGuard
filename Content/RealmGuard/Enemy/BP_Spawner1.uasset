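; BP_Spawner1 is the enemy wave spawner, reading each wave's groups from DT_Enemies by row name.
; ResetEnemy starts spawning; a delay loop spawns each group at its table transform, then advances to the next.
; DecreaseEnemy tracks survivors; once the last group is cleared, CurrentWave pays wave-scaled money, selects the next row and shows the start-wave widget.
; After the final wave, it pauses the game on a win screen.
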(event `self.ReceiveBeginPlay`
  (bind _asbp_third_person_character (cast `/Game/ThirdPerson/Blueprints/BP_ThirdPersonCharacter` (`GameplayStatics.GetPlayerCharacter` 0)))
  (set `self.As BP Third Person Character` _asbp_third_person_character))

(event `/Game/RealmGuard/Interfaces/BPI_Spawner.ResetEnemy`
  ;[1 1 1] Spawning Mechanics
  (set `self.Last Enemy?` false)
  (set `self.EnemySelector` 0)
  (if (== (`self.EnemiesAlive`) 0)
    (`KismetSystemLibrary.Delay` 0.2)
    (`/Game/RealmGuard/Interfaces/BPI_Spawner.Spawn`)))

(event `/Game/RealmGuard/Interfaces/BPI_Spawner.Spawn`
  (bind _enemyselector (`self.EnemySelector`))
  ;[1 1 1] Spawning Mechanics
  (bind _returnvalue (`|GetDataTableRow` "/Game/RealmGuard/Enemy/DataTable/DT_Enemies.DT_Enemies" (`self.Row Name`))
    (:`then`
      (bind (_enemy _numberofenemies _spawnlocation _delaybetween) (break `/Game/RealmGuard/Enemy/Structure/S_Enemies` _returnvalue))
      (set `self.Enemy` (`|GetArrayItem` _enemy _enemyselector))
      (`|ExecutionSequence`
        (:`then_0`
          (bind _output (`|GetArrayItem` _numberofenemies _enemyselector))
          (bind _output_get (set `self.EnemiesSpawned` _output))
          (`KismetSystemLibrary.Delay` (`|GetArrayItem` _delaybetween _enemyselector))
          (if (> _output_get 0) :!label _label
            (`KismetSystemLibrary.Delay` 1.0)
            (`|SpawnActorFromClass` (`self.Enemy`) (`|GetArrayItem` _spawnlocation _enemyselector) "Undefined" "MultiplyWithRoot" null null)
            (`/Engine/EditorBlueprintResources/StandardMacros.DecrementInt` (`self.EnemiesSpawned`)
              (:`  `
                (goto _label)))
            (else
              (`self.Enemy Selection`))))
        (:`then_1`
          (set `self.EnemiesAlive` (+ _output (`self.EnemiesAlive`))))))))

(event `Enemy Selection`
  ;[1 1 1] Spawning Mechanics
  (bind _result (`/Engine/EditorBlueprintResources/StandardMacros.IncrementInt` (`self.EnemySelector`))
    (:`  `
      (if (`KismetArrayLibrary.Array_IsValidIndex` (`.NumberofEnemies_6_7D1BE361433C38445C157B90C442BEF8` (break `/Game/RealmGuard/Enemy/Structure/S_Enemies` (stale `/Game/RealmGuard/Interfaces/BPI_Spawner.Spawn` _returnvalue))) _result)
        (`/Game/RealmGuard/Interfaces/BPI_Spawner.Spawn`)
        (else
          (set `self.Last Enemy?` true))))))

(event `CurrentWave`
  (bind _returnvalue (`GameplayStatics.GetPlayerController` 0))
  ;[1 1 1] Spawning Mechanics
  (if (< (`self.Wave`) 31)
    (`/Game/ThirdPerson/Blueprints/BP_ThirdPersonCharacter.Get Money` (`self.As BP Third Person Character`) (* (`self.Wave`) 25))
    (bind _result (`/Engine/EditorBlueprintResources/StandardMacros.IncrementInt` (`self.Wave`))
      (:`  `
        (set `self.Row Name` (`KismetStringLibrary.Conv_StringToName` (`KismetStringLibrary.Concat_StrStr` "Wave" (`KismetStringLibrary.Conv_IntToString` _result))))))
    (else
      ;;[1 1 1] Win Screen
      (cast `/Game/ThirdPerson/Blueprints/BP_ThirdPersonCharacter` (`GameplayStatics.GetPlayerCharacter` 0))
      (`WidgetLayoutLibrary.RemoveAllWidgets`)
      (bind _returnvalue_2 (`|GenericCreateObject` _returnvalue "/Game/RealmGuard/HUD/UI_GameWin.UI_GameWin_C"))
      (`UserWidget.AddToViewport` _returnvalue_2 0)
      (set `PlayerController.bShowMouseCursor` true _returnvalue)
      (`WidgetBlueprintLibrary.SetInputMode_UIOnlyEx` (`GameplayStatics.GetPlayerController` 0) null)
      (`GameplayStatics.SetGamePaused` true))))

(event `/Game/RealmGuard/Interfaces/BPI_Spawner.DecreaseEnemy`
  ;[1 1 1] Spawning Mechanics
  (bind _result (`/Engine/EditorBlueprintResources/StandardMacros.DecrementInt` (`self.EnemiesAlive`))
    (:`  `
      (bind _output_get (set `self.EnemiesAlive` _result))
      (if (and (== _output_get 0) (`self.Last Enemy?`))
        (`self.CurrentWave`)
        (`Widget.SetVisibility` (`/Game/ThirdPerson/Blueprints/BP_ThirdPersonCharacter.WB_StartWave` (`self.As BP Third Person Character`)) "Visible")))))

(fn `UserConstructionScript`)