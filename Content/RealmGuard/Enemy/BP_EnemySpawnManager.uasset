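; Spawner actor that releases goblin enemies in waves at its own location.
; StartWave starts a looping timer that spawns a BP_Goblin running BT_Goblin on each tick, ignoring collision.
; Each spawn increments the spawned count on the third-person game mode, and the timer is cleared once that count reaches the game mode's per-wave maximum.
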(event `self.ReceiveBeginPlay`
  (bind _asbp_third_person_game_mode (cast `/Game/ThirdPerson/Blueprints/BP_ThirdPersonGameMode` (`GameplayStatics.GetGameMode`)))
  (set `self.BP Third Person Game Mode` _asbp_third_person_game_mode))

(event `StartWave`
  (bind _returnvalue (`KismetSystemLibrary.K2_SetTimerDelegate` (delegate `SpawnEnemy`) (`self.EnemySpawnTime`) true))
  (set `self.SpanwEnemyTimerHandle` _returnvalue))

(event `SpawnEnemy`
  (bind _bp_third_person_game_mode (`self.BP Third Person Game Mode`))
  (`AIBlueprintHelperLibrary.SpawnAIFromClass` "/Game/RealmGuard/Enemy/BP_Goblin.BP_Goblin_C" "/Game/RealmGuard/Enemy/AI/BT_Goblin.BT_Goblin" (`self.K2_GetActorLocation`) (struct) true null)
  (bind _result (`/Engine/EditorBlueprintResources/StandardMacros.IncrementInt` (`/Game/ThirdPerson/Blueprints/BP_ThirdPersonGameMode.AmountOfEnemiesSpawnedThisWave` _bp_third_person_game_mode))
    (:`  `
      (if (>= _result (`/Game/ThirdPerson/Blueprints/BP_ThirdPersonGameMode.MaxEnemiesInWave` _bp_third_person_game_mode))
        (`KismetSystemLibrary.K2_ClearAndInvalidateTimerHandle` (`self.SpanwEnemyTimerHandle`))))))

(fn `UserConstructionScript`)