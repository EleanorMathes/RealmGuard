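; Level 3 area-of-effect turret in RealmGuard that calls meteors down on enemies.
; Tick continuously spins the Meteor component by RotationSpeed.
; When PawnSensing sees a BP_Enemy, a Delay paces the attack, then BP_Meteor spawns high above an enemy and a cast sound plays at the turret.
; The target comes from GetActorOfClass, so it is not necessarily the pawn that was seen.
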(event `self.ReceiveTick`
  (params (DeltaSeconds :type "Float (single-precision)"))
  (bind _meteor (`self.Meteor`))
  (`SceneComponent.K2_SetRelativeRotation` _meteor (`KismetMathLibrary.MakeRotator` 0.0 0.0 (+ (.yaw (.rotation (`SceneComponent.GetRelativeTransform` _meteor))) (`self.RotationSpeed`))) false false))

(event `self.PawnSensing.OnSeePawn`
  (params (Pawn :type "Pawn Object Reference"))
  (cast `/Game/RealmGuard/Enemy/BP_Enemy` Pawn)
  (`KismetSystemLibrary.Delay` 4.0)
  (bind _returnvalue (`GameplayStatics.GetActorOfClass` "/Game/RealmGuard/Enemy/BP_Enemy.BP_Enemy_C"))
  (`/Engine/EditorBlueprintResources/StandardMacros.IsValid` _returnvalue
    (:`Is Valid`
      (bind (_returnvalue_x _returnvalue_y _returnvalue_z) (`KismetMathLibrary.BreakVector` (`self.K2_GetActorLocation` _returnvalue)))
      (`|SpawnActorFromClass` "/Game/RealmGuard/Turret/BP_Meteor.BP_Meteor_C" (`KismetMathLibrary.MakeTransform` (`KismetMathLibrary.MakeVector` _returnvalue_x _returnvalue_y (+ _returnvalue_z 1000.0))) "Undefined" "MultiplyWithRoot" self null)
      (`GameplayStatics.PlaySoundAtLocation` "/Game/RealmGuard/SFX/Tower/Meteor_Cast.Meteor_Cast" (`self.K2_GetActorLocation`) (struct) 1.0 1.0 0.0 null null null null))))

(fn `UserConstructionScript`)