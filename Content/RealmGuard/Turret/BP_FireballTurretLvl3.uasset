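; BP_FireballTurretLvl3 is a level 3 turret that fires fireball projectiles when its pawn sensing spots an enemy.
; Seeing a BP_Enemy starts a one-second delay, which also throttles repeated sightings, then spawns a BP_FireballProjectile at one of three randomly chosen scene points.
; The projectile's target comes from GetActorOfClass, so it may differ from the enemy that was seen.
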(event `self.PawnSensing.OnSeePawn`
  (params (Pawn :type "Pawn Object Reference"))
  (cast `/Game/RealmGuard/Enemy/BP_Enemy` Pawn)
  (`KismetSystemLibrary.Delay` 1.0)
  (bind _returnvalue (`GameplayStatics.GetActorOfClass` "/Game/RealmGuard/Enemy/BP_Enemy.BP_Enemy_C"))
  (`|SpawnActorFromClass` "/Game/RealmGuard/Turret/BP_FireballProjectile.BP_FireballProjectile_C" (`SceneComponent.K2_GetComponentToWorld` (select `int` (`KismetMathLibrary.RandomIntegerInRange` 0 2) :`0` (`self.Scene`) :`1` (`self.Scene1`) :`2` (`self.Scene2`))) "Undefined" "MultiplyWithRoot" self _returnvalue null))

(fn `UserConstructionScript`)