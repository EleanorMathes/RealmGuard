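; Homing fireball projectile, fired by a turret judging by its folder, that damages enemies on contact.
; On BeginPlay, a valid Target sets the initial direction and rotation, becomes the ProjectileMovement homing target, and starts a timed self-destruct.
; Box overlap with a swept BP_Enemy hit spawns an explosion, destroys the projectile, then applies fixed damage to that enemy.
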(event `self.ReceiveBeginPlay`
  (`self.Target`
    (:`then`
      (`self.AimAtTarget`)
      (set `ProjectileMovementComponent.HomingTargetComponent` (`Actor.RootComponent` (`self.Target`)) (`self.ProjectileMovement`))
      (`KismetSystemLibrary.Delay` 10.0)
      (`self.K2_DestroyActor`))
    (:`else`)))

(event `AimAtTarget`
  (bind _output_get (set `MovementComponent.Velocity` (`KismetMathLibrary.GetDirectionUnitVector` (`self.K2_GetActorLocation`) (`self.K2_GetActorLocation` (`self.Target`))) (`self.ProjectileMovement`)))
  (`self.K2_SetActorRotation` (`KismetMathLibrary.Conv_VectorToRotator` _output_get)))

(event `self.Box.OnComponentBeginOverlap`
  (params (OverlappedComponent :type "PrimitiveComponent Object Reference") (OtherActor :type "Actor Object Reference") (OtherComp :type "PrimitiveComponent Object Reference") (OtherBodyIndex :type Integer) (bFromSweep :type Boolean) (SweepResult :type "HitResult Structure (by ref)"))
  (bind (_bblockinghit _binitialoverlap _time _distance _location _impactpoint _normal _impactnormal _physmat _hitactor) (`GameplayStatics.BreakHitResult` SweepResult))
  (bind _asbp_enemy (cast `/Game/RealmGuard/Enemy/BP_Enemy` _hitactor))
  (if (== _asbp_enemy _hitactor)
    (`GameplayStatics.SpawnEmitterAtLocation` "/Game/MilitaryWeapDark/FX/P_Grenade_Explosion_01.P_Grenade_Explosion_01" (`self.K2_GetActorLocation` _hitactor))
    (`self.K2_DestroyActor`)
    (`GameplayStatics.GetActorOfClass` "/Game/RealmGuard/Enemy/BP_Enemy.BP_Enemy_C")
    (`GameplayStatics.ApplyDamage` _hitactor 30.0)))

(fn `UserConstructionScript`)