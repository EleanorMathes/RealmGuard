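; BP_Base is the base structure in RealmGuard that loses health whenever a BP_Enemy reaches its hitbox.
; On overlap it calls DecreaseEnemyMessage on the player character, applies fixed damage to itself, spawns an explosion and destroys the enemy.
; The value returned by ApplyDamage is subtracted from BaseHealth and printed, and the base destroys itself once health runs out.
; The player HUD is cached at BeginPlay but not used.
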(event `self.ReceiveBeginPlay`
  (set `self.PlayerHUD` (`PlayerController.GetHUD` (`GameplayStatics.GetPlayerController` 0))))

(event `self.ReceiveTick`
  (params (DeltaSeconds :type "Float (single-precision)")))

(event `self.Hitbox.OnComponentBeginOverlap`
  (params (OverlappedComponent :type "PrimitiveComponent Object Reference") (OtherActor :type "Actor Object Reference") (OtherComp :type "PrimitiveComponent Object Reference") (OtherBodyIndex :type Integer) (bFromSweep :type Boolean) (SweepResult :type "HitResult Structure (by ref)"))
  (bind _basehealth (`self.BaseHealth`))
  (bind _asbp_enemy (cast `/Game/RealmGuard/Enemy/BP_Enemy` OtherActor))
  (message `/Game/RealmGuard/Interfaces/BPI_DecreaseEnemy.DecreaseEnemy` (`GameplayStatics.GetPlayerCharacter` 0))
  (bind _returnvalue (`GameplayStatics.ApplyDamage` self 5.0))
  (`GameplayStatics.SpawnEmitterAtLocation` "/Game/StarterContent/Particles/P_Explosion.P_Explosion" (`self.Location`) (struct) (10.0 10.0 10.0))
  (`self.K2_DestroyActor` _asbp_enemy)
  (if (> _basehealth 0.0)
    (bind _output_get (set `self.BaseHealth` (- _basehealth _returnvalue)))
    (`KismetSystemLibrary.PrintString` (`KismetStringLibrary.Conv_DoubleToString` _output_get))
    (if (<= _output_get 0.0)
      (`self.K2_DestroyActor`))))

(fn `UserConstructionScript`)