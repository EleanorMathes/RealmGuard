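; BP_Spike1 is a spike trap that damages actors other than the player character and wears out with use.
; When an actor begins overlapping Sphere1, the trap applies fixed damage to it, unless it is the first player's character.
; Each such overlap also takes one point off the trap's Health, and the trap destroys itself when that runs out.
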(event `self.Sphere1.OnComponentBeginOverlap`
  (params (OverlappedComponent :type "PrimitiveComponent Object Reference") (OtherActor :type "Actor Object Reference") (OtherComp :type "PrimitiveComponent Object Reference") (OtherBodyIndex :type Integer) (bFromSweep :type Boolean) (SweepResult :type "HitResult Structure (by ref)"))
  (if (!= OtherActor (`GameplayStatics.GetPlayerCharacter` 0))
    (`GameplayStatics.ApplyDamage` OtherActor 10.0)
    (set `self.Health` (- (`self.Health`) 1))
    (if (<= (`self.Health`) 0)
      (`self.K2_DestroyActor`))))

(fn `UserConstructionScript`)