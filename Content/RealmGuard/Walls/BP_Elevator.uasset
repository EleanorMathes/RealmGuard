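; BP_Elevator is an elevator that raises its platform when the player character enters its trigger box, then brings it back down.
; Separate MoveUp and MoveDown timelines drive the platform's relative location.
; A Disabled flag blocks retriggering until the cycle's delays elapse.
; Both delays hang off timeline Update pins rather than Finished, so they count from the start of each movement.
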(event `self.Box.OnComponentBeginOverlap`
  (params (OverlappedComponent :type "PrimitiveComponent Object Reference") (OtherActor :type "Actor Object Reference") (OtherComp :type "PrimitiveComponent Object Reference") (OtherBodyIndex :type Integer) (bFromSweep :type Boolean) (SweepResult :type "HitResult Structure (by ref)"))
  (if (== OtherActor (`GameplayStatics.GetPlayerCharacter` 0))
    (if (not (`self.Disabled?`))
      (bind (_direction _newtrack_1) (`Timeline|MoveUp` :!via `PlayFromStart`)
        (:`Update`
          (`SceneComponent.K2_SetRelativeLocation` (`self.Platform`) _newtrack_1 false false)
          (set `self.Disabled?` true)
          (`KismetSystemLibrary.Delay` 5.0)
          (bind (_direction_2 _newtrack_1_2) (`Timeline|MoveDown` :!via `PlayFromStart`)
            (:`Update`
              (`SceneComponent.K2_SetRelativeLocation` (`self.Platform`) _newtrack_1_2 false false)
              (`KismetSystemLibrary.Delay` 4.0)
              (set `self.Disabled?` false))))))))

(fn `UserConstructionScript`)